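; Player action that plays an idle break animation montage on the owning common character.
; When added, it sets a looping timer with a one-time random interval of a few minutes, which starts the action by its Action.IdleBreak tag through the owning component.
; The action stops itself when the montage completes, blends out or is interrupted.
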(event Custom|Start
  (bind _returnvalue (Class|CAction|GetOwningComponent))
  (Class|CActionComponent|StartActionbyTag _returnvalue (Components|GetOwner _returnvalue) "(TagName=\"Action.IdleBreak\")"))

(event EventStartAction
  (params (InInstigator :type Actor%20Object%20Reference))
  (bind _asccommon_character (Utilities|Casting|CastToCCommonCharacter (Components|GetOwner (Class|CAction|GetOwningComponent))))
  (Animation|Montage|PlayMontage (Variables|/Script/Engine.Character|GetMesh _asccommon_character) "/Game/CMP302/Meshes/Arms/Animation/New/AS_anim_idle_break_Montage.AS_anim_idle_break_Montage"
    (:OnCompleted
      _)
    (:OnBlendOut
      _)
    (:OnInterrupted
      _))
  (Class|CAction|StopAction InInstigator))

(event EventOnActionAdded
  (params (InInstigator :type Actor%20Object%20Reference))
  (Utilities|Time|SetTimerbyEvent (delegate Custom|Start) (Math|Random|RandomFloatinRange 1.5e+02 3e+02) true))