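; Enemy AI character that runs the BT_NormalEnemy behavior tree, with its logic held paused until BeginAILogic starts it.
; AI perception writes a sensed player to the blackboard with a line-of-sight flag from an eye-to-eye trace, and a short timer forgets the player after sensing is lost.
; TickAI turns the enemy to face the stored player.
; Taking a hit clears the player, stops the logic and unpossesses the controller.
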(event OnTargetPerceptionUpdated(AIPerception)
  (params (Actor :type Actor%20Object%20Reference) (Stimulus :type AI%20Stimulus%20Structure))
  (bind _self self)
  (bind _returnvalue (AI|GetAIController _self))
  (bind _returnvalue_2 (AI|GetBlackboard _returnvalue))
  ;[1 1 1] Perception Updated
  (if (Variables|Default|GetHasBeenInitialized)
    (if (.bSuccessfullySensed (Utilities|Struct|BreakAIStimulus Stimulus))
      (bind _ascplayer_character (Utilities|Casting|CastToCPlayerCharacter Actor))
      (Utilities|Time|ClearandInvalidateTimerbyHandle (Variables|Default|GetForgetPlayer_TimerHandle))
      (Utilities|IsValid _returnvalue_2
        (:Is%20Valid
          (AI|Components|Blackboard|SetValueasObject _returnvalue_2 (Variables|Default|GetPlayerName) _ascplayer_character)
          (Utilities|FlowControl|Delay 0.1)
          (bind _haslineofsight (CallFunction|CheckHasLineOfSight))
          (AI|Components|Blackboard|SetValueasBool _returnvalue_2 (Variables|Default|GetLineOfSight) _haslineofsight)))
      (else
        (bind _returnvalue_3 (Utilities|Time|SetTimerbyEvent (delegate Custom|ForgetPlayer) 2.0))
        (Variables|Default|SetForgetPlayer_TimerHandle _returnvalue_3)))))

(event Custom|ForgetPlayer
  (bind _self self)
  (bind _returnvalue (AI|GetAIController _self))
  (bind _returnvalue_2 (AI|GetBlackboard _returnvalue))
  ;[1 1 1] Perception Updated
  (Utilities|IsValid _returnvalue_2
    (:Is%20Valid
      (AI|Components|Blackboard|ClearValue _returnvalue_2 (Variables|Default|GetPlayerName))
      (AI|Components|Blackboard|SetValueasBool _returnvalue_2 (Variables|Default|GetLineOfSight) false))))

(event EventBeginAILogic
  (bind _self self)
  (bind _returnvalue (AI|GetAIController _self))
  (bind _braincomponent (Variables|/Script/AIModule.AIController|GetBrainComponent _returnvalue))
  ;[1 1 1] Init, Tick, HitTaken
  (Utilities|IsValid _returnvalue
    (:Is%20Valid
      (Utilities|IsValid _braincomponent
        (:Is%20Valid
          (AI|Logic|StartLogic _braincomponent))))))

(event EventTickAI
  (params (DeltaSeconds :type Float%20%28single-precision%29))
  (bind _returnvalue (Utilities|Name|MakeLiteralName "Player"))
  (bind _self self)
  (bind _returnvalue_2 (AI|GetAIController _self))
  (bind _returnvalue_3 (AI|GetBlackboard _returnvalue_2))
  (bind _returnvalue_4 (AI|Components|Blackboard|GetValueasObject _returnvalue_3 _returnvalue))
  ;[1 1 1] Init, Tick, HitTaken
  (if (Variables|Default|GetHasBeenInitialized)
    (Utilities|IsValid _returnvalue_2
      (:Is%20Valid
        (Utilities|IsValid _returnvalue_4
          (:Is%20Valid
            (bind _asactor (Utilities|Casting|CastToActor _returnvalue_4))
            (Transformation|SetActorRotation (Math|Rotator|MakeRotator 0.0 0.0 (.yaw (Math|Rotator|FindLookatRotation (Transformation|GetActorLocation) (Transformation|GetActorLocation _asactor)))))))))))

(event EventOnHitTakenBP
  (params (AttackData :type Attack%20Data%20Structure%20%28by%20ref%29))
  (bind _self self)
  (bind _returnvalue (AI|GetAIController _self))
  (bind _returnvalue_2 (AI|GetBlackboard _returnvalue))
  ;[1 1 1] Init, Tick, HitTaken
  (Utilities|IsValid _returnvalue_2
    (:Is%20Valid
      (AI|Components|Blackboard|ClearValue _returnvalue_2 (Utilities|Name|MakeLiteralName "Player"))
      (AI|Logic|StopLogic (Variables|/Script/AIModule.AIController|GetBrainComponent _returnvalue) "")
      (Utilities|Time|ClearandInvalidateTimerbyHandle (Variables|Default|GetForgetPlayer_TimerHandle))
      (Pawn|UnPossess (AI|GetAIController self)))))

(event EventInitAI
  (bind _self self)
  (bind _returnvalue (AI|GetAIController _self))
  ;[1 1 1] Init, Tick, HitTaken
  (AI|RunBehaviorTree _returnvalue "/Game/CMP302/Blueprints/AI/BT_NormalEnemy.BT_NormalEnemy")
  (AI|Logic|StopLogic (Variables|/Script/AIModule.AIController|GetBrainComponent _returnvalue) "")
  (bind _output_get (Variables|Default|SetHasBeenInitialized true))
  (Components|Tick|SetComponentTickEnabled (Variables|Default|GetAIPerception) _output_get))

(fn ConstructionScript)

(fn CheckHasLineOfSight
  (bind _self self)
  (bind _playername (Variables|Default|GetPlayerName))
  (bind _returnvalue (AI|GetAIController _self))
  (bind _returnvalue_2 (AI|GetBlackboard _returnvalue))
  (bind _returnvalue_3 (AI|Components|Blackboard|GetValueasObject _returnvalue_2 _playername))
  (Utilities|IsValid _returnvalue_2
    (:Is%20Valid
      (Utilities|IsValid _returnvalue_3
        (:Is%20Valid
          (bind _asactor (Utilities|Casting|CastToActor _returnvalue_3)
            (:then
              (LocalVariables|SetPlayerActor _asactor)
              (bind (_outhit _returnvalue_4) (Collision|LineTraceByChannel (.OutLocation (Actor|GetActorEyesViewPoint)) (.OutLocation (Actor|GetActorEyesViewPoint _asactor)) "TraceTypeQuery1" false 0 "None"))
              (if _returnvalue_4
                (return (== (.HitActor (Collision|BreakHitResult _outhit)) (LocalVariables|GetPlayerActor)))
                (else
                  (return true))))
            (:CastFailed
              (return false))))
        (:Is%20Not%20Valid
          (return false))))))