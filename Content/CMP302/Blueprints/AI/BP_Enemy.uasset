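; BP_Enemy is an AI enemy pawn that spots pawns by sight and turns to face its target.
; InitAI runs and restarts the BT_NormalEnemy behavior tree, while PawnSensing writes any seen pawn to the Blackboard's Player key.
; TickAI reads that key and snaps the enemy's yaw toward the target.
; OnHitTakenBP clears the key and stops the brain logic until it is started again.
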(event OnSeePawn(PawnSensing)
  (params (Pawn :type Pawn%20Object%20Reference))
  (bind _self self)
  (bind _returnvalue (AI|GetAIController _self))
  (bind _returnvalue_2 (AI|GetBlackboard _returnvalue))
  (Utilities|IsValid _returnvalue_2
    (:Is%20Valid
      (AI|Components|Blackboard|SetValueasObject _returnvalue_2 (Utilities|Name|MakeLiteralName "Player") Pawn))))

(event EventTickAI
  (params (DeltaSeconds :type Float%20%28single-precision%29))
  (bind _returnvalue (Utilities|Name|MakeLiteralName "Player"))
  (bind _self self)
  (bind _returnvalue_2 (AI|GetAIController _self))
  (bind _returnvalue_3 (AI|GetBlackboard _returnvalue_2))
  (bind _returnvalue_4 (AI|Components|Blackboard|GetValueasObject _returnvalue_3 _returnvalue))
  (Utilities|IsValid _returnvalue_2
    (:Is%20Valid
      (Utilities|IsValid _returnvalue_4
        (:Is%20Valid
          (bind _asactor (Utilities|Casting|CastToActor _returnvalue_4))
          (Transformation|SetActorRotation (Math|Rotator|MakeRotator 0.0 0.0 (.yaw (Math|Rotator|FindLookatRotation (Transformation|GetActorLocation) (Transformation|GetActorLocation _asactor))))))))))

(event EventOnHitTakenBP
  (params (AttackData :type Attack%20Data%20Structure%20%28by%20ref%29))
  (bind _self self)
  (bind _returnvalue (AI|GetAIController _self))
  (bind _returnvalue_2 (AI|GetBlackboard _returnvalue))
  (Utilities|IsValid _returnvalue_2
    (:Is%20Valid
      (AI|Components|Blackboard|SetValueasObject _returnvalue_2 (Utilities|Name|MakeLiteralName "Player") 0)
      (AI|Logic|StopLogic (Variables|/Script/AIModule.AIController|GetBrainComponent _returnvalue) ""))))

(event EventInitAI
  (bind _self self)
  (bind _returnvalue (AI|GetAIController _self))
  (bind _braincomponent (Variables|/Script/AIModule.AIController|GetBrainComponent _returnvalue))
  (AI|RunBehaviorTree _returnvalue "/Game/CMP302/Blueprints/AI/BT_NormalEnemy.BT_NormalEnemy")
  (AI|Logic|StartLogic _braincomponent)
  (Class|BrainComponent|RestartLogic _braincomponent))

(fn ConstructionScript)